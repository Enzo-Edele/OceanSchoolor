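; BP_Projectile is a colored shot from the squid game folder that homes in on a targeted shark.
; Launch tints the Niagara effect and sphere, then scales the timeline's play rate by distance to keep travel speed roughly constant.
; Each update lerps from the start transform to the shark's current one, passing strength to its Projectile function at 90%.
; It splashes and destroys itself on impact or if the target becomes invalid mid-flight.
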(event `Launch`
  (params (TargetedShark :type "/Game/Shark/BP_Shark Object Reference") (Color :type "Vector Structure") (Strenght :type "Float (double-precision)"))
  (bind _trajectory (`self.Trajectory`))
  (bind _returnvalue_location (`KismetMathLibrary.BreakTransform` (`self.GetTransform` (`self.Target`))))
  (`/Engine/EditorBlueprintResources/StandardMacros.IsValid` TargetedShark
    (:`Is Valid`
      (set `self.Target` TargetedShark)
      (set `self.ShootStrength` Strenght)
      (`FXSystemComponent.SetVectorParameter` (`self.NS_Projectile`) "Color" Color)
      (`MeshComponent.SetVectorParameterValueOnMaterials` (`self.Sphere`) "Color" Color)
      (`GameplayStatics.SpawnSound2D` "/Game/Sounds/Shoot_Cue.Shoot_Cue" 10.0 1.0 0.0 null)
      (bind _output_get (set `self.StartDest` (`self.GetTransform` self)))
      (`TimelineComponent.SetPlayRate` _trajectory (/ 1.0 (/ (* (`TimelineComponent.GetPlayRate` _trajectory) (`KismetMathLibrary.Vector_Distance` (.location _output_get) _returnvalue_location)) (`self.DistanceStd`))))
      (bind (_direction _alpha) (`Timeline|Trajectory`)
        (:`Update`
          (`/Engine/EditorBlueprintResources/StandardMacros.IsValid` (`self.Target`)
            (:`Is Valid`
              (if (>= _alpha 0.9)
                (`/Game/Shark/BP_Shark.Projectile` (`self.Target`) (`self.ShootStrength`))
                (`GameplayStatics.SpawnSound2D` "/Game/Sounds/Splash_Cue.Splash_Cue" 5.0 1.0 0.0 null :!label _label) ; set shark ncharge ds shark add charge
                (`self.K2_DestroyActor`)
                (else
                  (bind (_returnvalue_location_2 _returnvalue_rotation) (`KismetMathLibrary.BreakTransform` (`KismetMathLibrary.TLerp` (`self.StartDest`) (`self.GetTransform` (`self.Target`)) _alpha)))
                  (`self.K2_SetActorTransform` (`KismetMathLibrary.MakeTransform` _returnvalue_location_2 _returnvalue_rotation)))))
            (:`Is Not Valid`
              (goto _label))))))
    (:`Is Not Valid`
      (`self.K2_DestroyActor`))))

(fn `UserConstructionScript`)