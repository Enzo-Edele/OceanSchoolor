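; Clickable squid actor that owns the game camera, sets it as the view target and enables mouse clicks.
; Tick refills up to three charges at a Speed-scaled rate, showing each on a billboard through a material Progression parameter.
; Clicking the cube hands the squid to BP_GI for coloring, and right-click switches BP_GI to unselect mode.
; SetSquidColor stores the color and tints the cube's materials.
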(event `self.ReceiveBeginPlay`
  (bind _returnvalue (`GameplayStatics.GetPlayerController` 0))
  ;[1 1 1] Set First Cam
  (`PlayerController.SetViewTargetWithBlend` (`GameplayStatics.GetPlayerController` 0) (`self.Camera`) 0.0 "VTBlend_Linear" 0.0 false)
  ;[1 1 1] Make it Clickable
  (set `PlayerController.bEnableClickEvents` true _returnvalue)
  (set `PlayerController.bShowMouseCursor` true _returnvalue))

(event `self.ReceiveTick`
  (params (DeltaSeconds :type "Float (single-precision)"))
  ;[1 1 1] Reload Charge
  (if (< (`self.Charge`) 3.0)
    (bind _output_get (set `self.Charge` (+ (`self.Charge`) (* DeltaSeconds (* (`self.Speed`) 0.1)))))
    ;[1 1 1] Display Charge UI
    (`self.Set Charge Progression` (`self.Charge Left`) (`KismetMathLibrary.FClamp` _output_get))
    (`self.Set Charge Progression` (`self.Charge Middle`) (`KismetMathLibrary.FClamp` (- _output_get 1.0)))
    (`self.Set Charge Progression` (`self.Charge Right`) (- _output_get 2.0))))

(event `self.Cube.OnClicked`
  (params (TouchedComponent :type "PrimitiveComponent Object Reference") (ButtonPressed :type "Key Structure"))
  ;[1 1 1] Handle Control
  (bind _asbp_gi (cast `/Game/BP_GI` (`GameplayStatics.GetGameInstance`)))
  (`/Game/BP_GI.SetSquidColor` _asbp_gi self))

(event `Key|RightMouseButton`
  (params (Key :type "Key Structure"))
  ;[1 1 1] None Selected Mode
  (:`Pressed`
    (bind _asbp_gi (cast `/Game/BP_GI` (`GameplayStatics.GetGameInstance`)))
    (`/Game/BP_GI.ChangeMode` :`self` _asbp_gi :`UnselectMode` true)
    (`KismetSystemLibrary.PrintString` "r clic")))

(fn `Set Charge Progression`
  (params (`Charge Billboard` :type "PrimitiveComponent Object Reference") (`Charge Value` :type "Float (single-precision)"))
  (bind _returnvalue (`PrimitiveComponent.CreateDynamicMaterialInstance` `Charge Billboard` 0 null "None"))
  (`MaterialInstanceDynamic.SetScalarParameterValue` _returnvalue "Progression" `Charge Value`))

(fn `Set Squid Color`
  (params (`New Color` :type "/Game/LevelData/ColorStruct Structure"))
  (bind _output_get (set `self.SquidColor` `New Color`))
  ;[1 1 1] Render Color
  (`MeshComponent.SetVectorParameterValueOnMaterials` (`self.Cube`) "Color" (`.ColorVector_7_4A9F842A4BB80A4C8A19C28782F34C3B` (break `/Game/LevelData/ColorStruct` _output_get))))

(fn `UserConstructionScript`)