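; BP_Shark_Fred is a placeholder shark Blueprint that colors its Cylinder, Cube and Cone meshes from a data table.
; Every Tick, it pushes the stored Color vector to the "Color" material parameter on all three meshes.
; It then looks up ColorName in the Data table and stores the row for the next frame, printing a message when the row is missing.
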(event `self.ReceiveTick`
  (params (DeltaSeconds :type "Float (single-precision)"))
  (bind (_color_colorname _color_colorvector) (break `/Game/LevelData/ColorStruct` (`self.Color`)))
  ;[1 1 1] Change la couleur du material
  (`MeshComponent.SetVectorParameterValueOnMaterials` (`self.Cylinder`) "Color" _color_colorvector)
  (`MeshComponent.SetVectorParameterValueOnMaterials` (`self.Cube`) "Color" _color_colorvector)
  (`MeshComponent.SetVectorParameterValueOnMaterials` (`self.Cone`) "Color" _color_colorvector)
  (bind _returnvalue (`|GetDataTableRow` (`self.Data`) (`self.ColorName`))
    (:`then`
      (set `self.Color` _returnvalue))
    (:`RowNotFound`
      (`KismetSystemLibrary.PrintString` "Row Not Found" true true (struct :`G` 0.66 :`B` 1.0 :`A` 1.0) 0.0))))

(fn `UserConstructionScript`)