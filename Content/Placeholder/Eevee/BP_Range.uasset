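; BP_Range is a Blueprint that builds an open cylinder side wall as a procedural mesh in its Construction Script, likely as a range visual.
; CreateCylinder places bottom and top vertex rings from Radius, Height, HeightOffset and Detail, stitches quads with wrapped UVs, and computes normals and tangents.
; The section is then created and given Material.
; A flat-disc CreateCircle function also exists but is not called by the Construction Script.
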(fn `Clear Mesh Data`
  (`KismetArrayLibrary.Array_Clear` (`self.Vertices`))
  (`KismetArrayLibrary.Array_Clear` (`self.Triangles`))
  (`KismetArrayLibrary.Array_Clear` (`self.Normals`))
  (`KismetArrayLibrary.Array_Clear` (`self.UV0`))
  (`KismetArrayLibrary.Array_Clear` (`self.Tangents`)))

(fn `Create Circle`
  (bind (_cos_x_ _sin_y_) (`self.Calculate Angle with Distance` 1))
  (set `self.Vertices` (`|MakeArray` (0.0 0.0 0.0) (`KismetMathLibrary.MakeVector` _cos_x_ _sin_y_) :!type "Vector Structure"))
  (for _index (range (+ (- (`self.Detail`) 2) 1))
    (bind _returnvalue (+ _index 2))
    (bind (_cos_x__2 _sin_y__2) (`self.Calculate Angle with Distance` _returnvalue))
    ;[1 1 1] Add Vertex
    (`KismetArrayLibrary.Array_Add` (`self.Vertices`) (`KismetMathLibrary.MakeVector` _cos_x__2 _sin_y__2))
    ;[1 1 1] Add Triangle
    (`self.Add Triangle For Circle` _returnvalue (+ _index 1)))
  ;[1 1 1] Add Last Triangle
  (`self.Add Triangle For Circle` 1 (`self.Detail`))
  ;[1 1 1] Add Uv Center
  (`KismetArrayLibrary.Array_Add` (`self.UV0`) (0.5 0.5))
  ;[1 1 1] Add Uvs
  (for _index_2 (range 1 (+ (`self.Detail`) 1))
    (bind (_cos_x__3 _sin_y__3) (`self.Calculate Angle` _index_2))
    (`KismetArrayLibrary.Array_Add` (`self.UV0`) (`KismetMathLibrary.MakeVector2D` (+ (* _cos_x__3 0.5) 0.5) (+ (* _sin_y__3 0.5) 0.5))))
  ;[1 1 1] Calculate Tanget + Normals
  (bind (_normals _tangents) (`KismetProceduralMeshLibrary.CalculateTangentsForMesh` (`self.Vertices`) (`self.Triangles`) (`self.UV0`)))
  (set `self.Normals` _normals)
  (set `self.Tangents` _tangents))

(fn `Create Cylinder`
  (bind _uv0 (`self.UV0`))
  (bind _uv0_2 (`self.UV0`))
  (`|ExecutionSequence`
    (:`then_0`
      ;[1 1 1] Add Vertices
      (for _index (range (+ (`self.Detail`) 1))
        (bind (_cos_x_ _sin_y_) (`self.Calculate Angle with Distance` _index))
        (`KismetArrayLibrary.Array_Add` (`self.Vertices`) (`KismetMathLibrary.MakeVector` _cos_x_ _sin_y_ (+ (* -0.5 (`self.Height`)) (`self.HeightOffset`))))
        (`KismetArrayLibrary.Array_Add` (`self.Vertices`) (`KismetMathLibrary.MakeVector` _cos_x_ _sin_y_ (+ (* 0.5 (`self.Height`)) (`self.HeightOffset`))))))
    (:`then_1`
      (for _index_2 (range (`self.Detail`))
        ;[1 1 1] Add Triangles
        (`self.Add Triangle for Cylinder (Loop)` (* _index_2 2))
        (bind _returnvalue (/ _index_2 (`KismetMathLibrary.Conv_IntToDouble` (`self.Detail`))))
        ;[1 1 1] Add UVs
        (`KismetArrayLibrary.Array_Add` _uv0 (`KismetMathLibrary.MakeVector2D` _returnvalue 1.0))
        (`KismetArrayLibrary.Array_Add` _uv0 (`KismetMathLibrary.MakeVector2D` _returnvalue)))
      ;[1 1 1] Add last UV
      (`KismetArrayLibrary.Array_Add` _uv0_2 (1.0 1.0))
      (`KismetArrayLibrary.Array_Add` _uv0_2 (1.0 0.0)))
    (:`then_2`
      ;[1 1 1] Calculate Tanget + Normals
      (bind (_normals _tangents) (`KismetProceduralMeshLibrary.CalculateTangentsForMesh` (`self.Vertices`) (`self.Triangles`) (`self.UV0`)))
      (set `self.Normals` _normals)
      (set `self.Tangents` _tangents))))

(fn `UserConstructionScript`
  (`self.Clear Mesh Data`)
  (`|ExecutionSequence`
    (:`then_0`
      (`self.Create Cylinder`))
    (:`then_1`
      (`ProceduralMeshComponent.CreateMeshSection_LinearColor` :`self` (`self.ProceduralMesh`) :`Vertices` (`self.Vertices`) :`Triangles` (`self.Triangles`) :`Normals` (`self.Normals`) :`UV0` (`self.UV0`) :`Tangents` (`self.Tangents`))
      (`PrimitiveComponent.SetMaterial` (`self.ProceduralMesh`) 0 (`self.Material`)))))