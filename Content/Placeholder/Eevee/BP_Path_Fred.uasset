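; BP_Path_Fred is a spline path actor that moves registered sharks along its length.
; AddShark fills the Sharks list; each Tick advances every shark's distance by Speed plus DeltaSeconds (added, not multiplied) and stores its progress fraction.
; Sharks are placed on the spline and face its end point with a -90 degree rotation offset, rather than following the tangent.
; Sharks past the end only trigger an "Arrivé" debug print.
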(event `Add Shark`
  (params (`New Shark` :type "/Game/Placeholder/Eevee/BP_Shark_Fred Object Reference"))
  (`KismetArrayLibrary.Array_Add` (`self.Sharks`) `New Shark`))

(event `self.ReceiveTick`
  (params (DeltaSeconds :type "Float (single-precision)"))
  (bind _spline (`self.Spline`))
  ;[1 1 1] Vérif si la liste n'est pas nul
  (if (not (== 0 (`KismetArrayLibrary.Array_Length` (`self.Sharks`))))
    (for _array_element (`self.Sharks`)
      (bind _distanceparcouru (`/Game/Placeholder/Eevee/BP_Shark_Fred.DistanceParcouru` _array_element))
      (if (<= _distanceparcouru (`SplineComponent.GetSplineLength` (`self.Spline`)))
        ;[1 1 1] Calcule la prochaine pos du requin
        (bind _output_get (set `/Game/Placeholder/Eevee/BP_Shark_Fred.DistanceParcouru` (+ _distanceparcouru (+ (`/Game/Placeholder/Eevee/BP_Shark_Fred.Speed` _array_element) DeltaSeconds)) _array_element))
        ;[1 1 1] Set Distance %
        (set `/Game/Placeholder/Eevee/BP_Shark_Fred.Distance%` (/ _output_get (`SplineComponent.GetSplineLength` (`self.Spline`))) _array_element)
        (bind _returnvalue (`SplineComponent.GetLocationAtDistanceAlongSpline` (`self.Spline`) _output_get "World"))
        (`self.K2_SetActorLocation` _array_element _returnvalue false false)
        (`self.K2_SetActorRotation` _array_element (`KismetMathLibrary.ComposeRotators` (struct :`Pitch` -90.0) (`KismetMathLibrary.FindLookAtRotation` _returnvalue (`SplineComponent.GetLocationAtSplinePoint` _spline (`SplineComponent.GetNumberOfSplinePoints` _spline) "World"))) false)
        (else
          (`KismetSystemLibrary.PrintString` "Arrivé" true true (struct :`G` 0.66 :`B` 1.0 :`A` 1.0) 0.0))))))

(fn `UserConstructionScript`)