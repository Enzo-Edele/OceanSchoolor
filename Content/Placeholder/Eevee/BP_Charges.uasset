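; BP_Charges is a placeholder charge indicator that shows the Squid's current Charge as up to three material billboards.
; On BeginPlay it hides the direct child components of its ChildActor component.
; Every Tick it polls Squid.Charge and sets each billboard's visibility against rising thresholds.
; The first two billboards appear on reaching their threshold, while the third requires Charge to strictly exceed its threshold.
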(event `self.ReceiveBeginPlay`
  (for _array_element (`SceneComponent.GetChildrenComponents` (`self.ChildActor`) false)
    (`SceneComponent.SetHiddenInGame` _array_element true false)))

(event `self.ReceiveTick`
  (params (DeltaSeconds :type "Float (single-precision)"))
  (bind _charge (`/Game/Edele/BP_Pawn_Squid.Charge` (`self.Squid`)))
  (`SceneComponent.SetHiddenInGame` (`self.MaterialBillboard`) (> 1.0 _charge) false)
  (`SceneComponent.SetHiddenInGame` (`self.MaterialBillboard1`) (> 2.0 _charge) false)
  (`SceneComponent.SetHiddenInGame` (`self.MaterialBillboard2`) (>= 3.0 _charge) false))

(fn `UserConstructionScript`)