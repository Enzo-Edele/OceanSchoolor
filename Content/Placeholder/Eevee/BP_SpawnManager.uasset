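; BP_SpawnManager is a placeholder actor that spawns BP_Shark actors on a timed schedule from its SpawnList.
; On BeginPlay it insertion-sorts the list by SpawnTime, which a French author note flags as unoptimized.
; Each Tick it spawns at most one due shark at OutRangeTransform, sets its color, and hands it to the entry's path via AddShark.
; It destroys itself after the last entry.
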(event `self.ReceiveBeginPlay`
  ;[1 1 1] Tri insertion, non optimisé
  (`self.SortSpawnList`))

(event `self.ReceiveTick`
  (params (DeltaSeconds :type "Float (single-precision)"))
  (bind _output_spawntime (break `/Game/Placeholder/Eevee/SpawnStruct` (`|GetArrayItem` (`self.SpawnList`) (`self.Current`))))
  (bind (_output_spawntime_2 _output_path _output_sharktype _output_sharkcolor) (break `/Game/Placeholder/Eevee/SpawnStruct` (`|GetArrayItem` (`self.SpawnList`) (`self.Current`))))
  (if (<= _output_spawntime (`self.GetGameTimeSinceCreation`))
    (bind _returnvalue (`|SpawnActorFromClass` "/Game/Placeholder/Eevee/BP_Shark.BP_Shark_C" (`self.OutRangeTransform`) "Undefined" "OverrideRootScale" null null))
    (set `/Game/Placeholder/Eevee/BP_Shark.ColorName` _output_sharkcolor _returnvalue)
    (`/Game/Placeholder/Eevee/BP_Path.Add Shark` (`|GetArrayItem` (`self.Paths`) _output_path) _returnvalue)
    (if (< (`self.Current`) (- (`KismetArrayLibrary.Array_Length` (`self.SpawnList`)) 1))
      (`/Engine/EditorBlueprintResources/StandardMacros.IncrementInt` (`self.Current`))
      (else
        (`self.K2_DestroyActor`)))))

(fn `UserConstructionScript`)