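; Clickable pedestal where the player places squids, signalling when it is free during the Preparation state.
; Binds to the level instance's click-mode and state-change events through BP_GI, waiting for that instance's creation if needed.
; A self-restarting timeline pulses the material toward SquidColor and animates an arrow while squids remain and the pedestal is unoccupied.
; An incoming wave clears the highlight, and clicks pass the pedestal to the level instance's PlaceSquid.
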(event `self.ReceiveBeginPlay`
  (bind _asbp_gi (cast `/Game/Scripts/BP_GI` (`GameplayStatics.GetGameInstance`)))
  (`/Engine/EditorBlueprintResources/StandardMacros.IsValid` (`/Game/Scripts/BP_GI.Level Instance` _asbp_gi)
    (:`Is Valid`
      (`self.OnLICreated`))
    (:`Is Not Valid`
      (add `/Game/Scripts/BP_GI.OnLevelInstanceCreated` _asbp_gi (delegate `OnLICreated`)))))

(event `Unbind`
  (params (`Level Instance` :type "/Game/Scripts/BP_LI Object Reference"))
  (remove `/Game/Scripts/BP_LI.OnClickModeChange` `Level Instance` (delegate `HighLightPedestal`))
  (remove `/Game/Scripts/BP_LI.OnLevelStateChanged` `Level Instance` (delegate `HighLightPedestal`)))

(event `OnLICreated`
  (bind _asbp_gi (cast `/Game/Scripts/BP_GI` (`GameplayStatics.GetGameInstance`)))
  (bind _level_instance (`/Game/Scripts/BP_GI.Level Instance` _asbp_gi))
  (add `/Game/Scripts/BP_LI.OnClickModeChange` _level_instance (delegate `HighLightPedestal`))
  (add `/Game/Scripts/BP_LI.OnLevelStateChanged` _level_instance (delegate `HighLightPedestal`)))

(event `HighLightPedestal`
  (bind (_arrowstartpos_x _arrowstartpos_y _arrowstartpos_z) (`KismetMathLibrary.BreakVector` (`self.ArrowStartPos`)))
  (bind _asbp_gi (cast `/Game/Scripts/BP_GI` (`GameplayStatics.GetGameInstance`)))
  (bind _level_instance (`/Game/Scripts/BP_GI.Level Instance` _asbp_gi))
  (switch `/Game/Scripts/LevelState` (`/Game/Scripts/BP_LI.CurrentState` _level_instance)
    (:`NewEnumerator1`
      (if (and (> (`/Game/Scripts/BP_LI.NbSquid` _level_instance) 0) (== (`self.Occupied`) false) (== (`TimelineComponent.IsPlaying` (`self.Highlight`)) false))
        (`SceneComponent.SetHiddenInGame` (`self.PedestalArrow`) false false)
        (set `self.ArrowStartPos` (`SceneComponent.RelativeLocation` (`self.PedestalArrow`)))
        (bind (_direction _t) (`Timeline|Highlight` :!via `PlayFromStart` :!label _label)
          (:`Update`
            (`MeshComponent.SetVectorParameterValueOnMaterials` (`self.Pedestal`) "Color" (`KismetMathLibrary.VLerp` (0.0 0.0 0.0) (`self.SquidColor`) _t))
            (`SceneComponent.K2_SetRelativeLocation` (`self.PedestalArrow`) (`KismetMathLibrary.MakeVector` _arrowstartpos_x _arrowstartpos_y (`KismetMathLibrary.Lerp` _arrowstartpos_z (+ _arrowstartpos_z 100.0) _t)) false false))
          (:`Finished`
            (if (`self.Occupied`)
              (`SceneComponent.SetHiddenInGame` (`self.PedestalArrow`) true false :!label _label_2)
              (else
                (goto _label :!via `PlayFromStart`)))))))
    (:`NewEnumerator2`
      (`TimelineComponent.Stop` (`self.Highlight`))
      (`MeshComponent.SetVectorParameterValueOnMaterials` (`self.Pedestal`) "Color" (0.0 0.0 0.0))
      (goto _label_2))))

(event `ChangeColor`
  (params (`New Color` :type "Vector Structure"))
  (`MeshComponent.SetVectorParameterValueOnMaterials` (`self.Pedestal`) "Color" `New Color`))

(event `self.Pedestal.OnClicked`
  (params (TouchedComponent :type "PrimitiveComponent Object Reference") (ButtonPressed :type "Key Structure"))
  ;[1 1 1] Place Squid
  (bind _asbp_gi (cast `/Game/Scripts/BP_GI` (`GameplayStatics.GetGameInstance`)))
  (`/Game/Scripts/BP_LI.Place Squid` (`/Game/Scripts/BP_GI.Level Instance` _asbp_gi) self (`self.Occupied`)))

(fn `UserConstructionScript`)