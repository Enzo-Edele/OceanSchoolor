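; Game instance blueprint that holds the player's current interaction mode (squid, pearl, shot or no select) for a squid-and-shark color matching game.
; ChangeMode sets the mode flags, selected color and mode text.
; Squid mode spawns squids on free pedestals; pearl mode recolors a squid, then possesses it and enters shot mode, keeping the stored camera as view target.
; Shots spend squid charge and return whether its color matches the shark's desired color.
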(fn `Camera`
  (params (Cam :type "Actor Object Reference"))
  (set `self.Cam` Cam)
  (return))

(fn `ChangeMode`
  (params (SquidMode :type Boolean) (PearlMode :type Boolean) (ShotMode :type Boolean) (UnselectMode :type Boolean) (Color :type "/Game/LevelData/ColorStruct Structure"))
  (bind _output_get (set `self.SquidMode` SquidMode))
  (if _output_get
    (set `self.ModeText` "Squid"))
  (bind _output_get_2 (set `self.PearlMode` PearlMode))
  (if _output_get_2
    (set `self.PearlSelected` Color)
    (set `self.ModeText` "Pearl"))
  (bind _output_get_3 (set `self.ShotMode` ShotMode))
  (if _output_get_3
    (set `self.ModeText` "Shot")
    (set `self.SquidSelectedColor` Color))
  (bind _output_get_4 (set `self.UnselectMode` UnselectMode))
  (if _output_get_4
    (set `self.ModeText` "No select")))

(fn `ControlSquid`
  (params (Squid :type "Actor Object Reference"))
  (bind _returnvalue (`GameplayStatics.GetPlayerController` 0))
  (bind _aspawn (cast `Pawn` Squid))
  (`Controller.UnPossess` _returnvalue)
  (`Controller.Possess` _returnvalue _aspawn)
  (`PlayerController.SetViewTargetWithBlend` (`GameplayStatics.GetPlayerController` 0) (`self.Cam`) 0.0 "VTBlend_Linear" 0.0 false)
  (bind _asbp_squid (cast `/Game/Squid/BP_Squid` (`local.Squid`)))
  (`self.ChangeMode` false false true false (`/Game/Squid/BP_Squid.SquidColor` _asbp_squid))
  (bind _output_get (set `self.SquidControl` (`local.Squid`)))
  (`KismetSystemLibrary.PrintString` (`KismetSystemLibrary.GetObjectName` _output_get))
  (return))

(fn `PlaceSquid`
  (params (Pedestal :type "/Game/Squid/BP_Pedestal Object Reference") (`Pedestal Occupied` :type Boolean))
  (bind _returnvalue (`Actor.GetTransform` (`local.Pedestal`)))
  ;[1 1 1] Check Mode
  (if (`self.SquidMode`)
    ;[1 1 1] Check Placed
    (if `Pedestal Occupied`
      ;[1 1 1] Already Placed
      (`KismetSystemLibrary.PrintString` "Already Placed")
      (return)
      (else
        ;[1 1 1] Spawn Actor
        (`|SpawnActorFromClass` (`self.SquidPrefab`) (`KismetMathLibrary.MakeTransform` (`KismetMathLibrary.MakeVector` (.x (.location _returnvalue)) (.y (.location _returnvalue)) (+ (.z (.location _returnvalue)) (`/Game/Squid/BP_Pedestal.SquidOffset` (`local.Pedestal`)))) (.rotation _returnvalue) (.scale _returnvalue)) "Undefined" "OverrideRootScale" null null)
        ;[1 1 1] Camera Things
        (`PlayerController.SetViewTargetWithBlend` (`GameplayStatics.GetPlayerController` 0) (`self.Cam`) 0.0 "VTBlend_Linear" 0.0 false)
        (`KismetSystemLibrary.PrintString` "SpawnSquid")
        (return)))))

(fn `Set text`
  (returns (nT :type Text))
  (return (`self.ModeText`)))

(fn `SetSquidColor`
  (params (Squid :type "Actor Object Reference"))
  ;[1 1 1] Check Mode
  (if (`self.PearlMode`)
    ;[1 1 1] Good mode
    (bind _asbp_squid (cast `/Game/Squid/BP_Squid` Squid))
    (`/Game/Squid/BP_Squid.Set Squid Color` _asbp_squid (`self.PearlSelected`))
    (`self.ControlSquid` (`local.Squid`))
    (`KismetSystemLibrary.PrintString` "Change")
    (return)
    (else
      ;[1 1 1] Not a good mode
      (`KismetSystemLibrary.PrintString` "no change")
      (return))))

(fn `ShotShark`
  (params (`Shot Shark` :type "Actor Object Reference") (DesireColor :type "/Game/LevelData/ColorStruct Structure"))
  (returns (Matched :type Boolean))
  (bind _desirecolor (`local.DesireColor`))
  (bind _desirecolor_2 (`local.DesireColor`))
  (bind _squidselectedcolor (`self.SquidSelectedColor`))
  (bind _squidselectedcolor_2 (`self.SquidSelectedColor`))
  (bind _desirecolor_colorname (break `/Game/LevelData/ColorStruct` (`local.DesireColor`)))
  (bind _squidselectedcolor_colorname (break `/Game/LevelData/ColorStruct` (`self.SquidSelectedColor`)))
  (bind _returnvalue (== _desirecolor_colorname _squidselectedcolor_colorname))
  ;[1 1 1] Check Mode
  (if (`self.ShotMode`)
    (bind _asbp_squid (cast `/Game/Squid/BP_Squid` (`self.SquidControl`)))
    (bind _charge (`/Game/Squid/BP_Squid.Charge` _asbp_squid))
    ;[1 1 1] Handle Charge
    (if (> _charge 1.0)
      (set `/Game/Squid/BP_Squid.Charge` (- _charge 1.0) _asbp_squid)
      ;[1 1 1] Check Color Match
      (if _returnvalue
        ;[1 1 1] Color Match
        (`KismetSystemLibrary.PrintString` "happy shork" true true (make `LinearColor` (.x (`.ColorVector_7_4A9F842A4BB80A4C8A19C28782F34C3B` (break `/Game/LevelData/ColorStruct` _desirecolor_2))) (.y (`.ColorVector_7_4A9F842A4BB80A4C8A19C28782F34C3B` (break `/Game/LevelData/ColorStruct` _desirecolor_2))) (.z (`.ColorVector_7_4A9F842A4BB80A4C8A19C28782F34C3B` (break `/Game/LevelData/ColorStruct` _desirecolor_2)))))
        (`KismetSystemLibrary.PrintString` "Good Color" true true (make `LinearColor` (.x (`.ColorVector_7_4A9F842A4BB80A4C8A19C28782F34C3B` (break `/Game/LevelData/ColorStruct` _squidselectedcolor_2))) (.y (`.ColorVector_7_4A9F842A4BB80A4C8A19C28782F34C3B` (break `/Game/LevelData/ColorStruct` _squidselectedcolor_2))) (.z (`.ColorVector_7_4A9F842A4BB80A4C8A19C28782F34C3B` (break `/Game/LevelData/ColorStruct` _squidselectedcolor_2)))))
        (else
          ;[1 1 1] Color Not Match
          (`KismetSystemLibrary.PrintString` "angry shaaark" true true (make `LinearColor` (.x (`.ColorVector_7_4A9F842A4BB80A4C8A19C28782F34C3B` (break `/Game/LevelData/ColorStruct` _desirecolor))) (.y (`.ColorVector_7_4A9F842A4BB80A4C8A19C28782F34C3B` (break `/Game/LevelData/ColorStruct` _desirecolor))) (.z (`.ColorVector_7_4A9F842A4BB80A4C8A19C28782F34C3B` (break `/Game/LevelData/ColorStruct` _desirecolor)))))
          (`KismetSystemLibrary.PrintString` "Bad Color" true true (make `LinearColor` (.x (`.ColorVector_7_4A9F842A4BB80A4C8A19C28782F34C3B` (break `/Game/LevelData/ColorStruct` _squidselectedcolor))) (.y (`.ColorVector_7_4A9F842A4BB80A4C8A19C28782F34C3B` (break `/Game/LevelData/ColorStruct` _squidselectedcolor))) (.z (`.ColorVector_7_4A9F842A4BB80A4C8A19C28782F34C3B` (break `/Game/LevelData/ColorStruct` _squidselectedcolor)))))))
      (return _returnvalue))))