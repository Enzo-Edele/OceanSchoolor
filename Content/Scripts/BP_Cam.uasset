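; BP_Cam is a camera Blueprint that registers itself as the camera of the level instance held by BP_GI, the game instance.
; On BeginPlay it calls SetCam at once if the level instance is valid, otherwise it binds SetCam to the game instance's OnLevelInstanceCreated event.
; SetCam passes the Blueprint itself to the level instance's SetCamera, so registration also works when the level instance is created later.
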(event `self.ReceiveBeginPlay`
  (bind _asbp_gi (cast `/Game/Scripts/BP_GI` (`GameplayStatics.GetGameInstance`)))
  (`/Engine/EditorBlueprintResources/StandardMacros.IsValid` (`/Game/Scripts/BP_GI.Level Instance` _asbp_gi)
    (:`Is Valid`
      (`self.Set Cam`))
    (:`Is Not Valid`
      (add `/Game/Scripts/BP_GI.OnLevelInstanceCreated` _asbp_gi (delegate `Set Cam`)))))

(event `Set Cam`
  (bind _asbp_gi (cast `/Game/Scripts/BP_GI` (`GameplayStatics.GetGameInstance`)))
  (`/Game/Scripts/BP_LI.Set Camera` (`/Game/Scripts/BP_GI.Level Instance` _asbp_gi) self))

(fn `UserConstructionScript`)