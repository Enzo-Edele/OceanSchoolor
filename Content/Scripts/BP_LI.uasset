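; BP_LI is the level manager for a squid-versus-shark defense game, registering with BP_GI and tracking level state and click mode.
; During preparation and waves, players place squids on pedestals, recolor them with pearls and select one to shoot.
; ShootShark returns an outcome enum from charge, range and color match, with full charge bypassing range.
; Squid stock doubles as mermaid lives, and event dispatchers broadcast changes.
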(event `self.ReceiveBeginPlay`
  ;[1 1 1] Init
  (bind _asbp_gi (cast `/Game/Scripts/BP_GI` (`GameplayStatics.GetGameInstance`)))
  (`/Game/Scripts/BP_GI.Set Level Instance` _asbp_gi self)
  (`/Game/Scripts/BP_GI.SetUMG` _asbp_gi "NewEnumerator2")
  (`self.Set Current State` "NewEnumerator0")
  (`self.EnableInput` (`GameplayStatics.GetPlayerController` 0))
  (bind _returnvalue (`GameplayStatics.SpawnSound2D` (`self.LevelSound`) 1.0 1.0 0.0 null))
  (`AudioComponent.Play` _returnvalue 0.0))

(event `Key|RightMouseButton`
  (params (Key :type "Key Structure"))
  ;[1 1 1] UnSelected Mode
  (:`Pressed`
    (`self.Change Mode` "NewEnumerator3")))

(fn `Change Mode`
  (params (Mode :type "/Game/Scripts/ClickMode Enum" :default "NewEnumerator0") (Color :type "/Game/Scripts/ColorStruct Structure"))
  (set `self.PreviousMode` (`self.CurrentMode`))
  (bind _output_get (set `self.CurrentMode` (`local.Mode`)))
  (switch `/Game/Scripts/ClickMode` _output_get
    (:`NewEnumerator3`
      _)
    (:`NewEnumerator0`
      _)
    (:`NewEnumerator1`
      (set `self.SelectedPearl` (`local.Color`)))
    (:`NewEnumerator2`
      (set `self.SelectedSquidColor` (`local.Color`))))
  (`self.OnClickModeChange`))

(fn `ControlSquid`
  (params (Squid :type "/Game/Squid/BP_Squid Object Reference"))
  (bind _squidcontrol (`self.SquidControl`))
  (switch `/Game/Scripts/LevelState` (`self.CurrentState`)
    (:`NewEnumerator1`
      _)
    (:`NewEnumerator2`
      _))
  (`self.Change Mode` "NewEnumerator2" (`/Game/Squid/BP_Squid.SquidColor` (`local.Squid`)))
  (`/Engine/EditorBlueprintResources/StandardMacros.IsValid` _squidcontrol
    (:`Is Valid`
      (`/Game/Squid/BP_Squid.Hide Ring` _squidcontrol true))
    (:`Is Not Valid`
      _))
  (set `self.SquidControl` (`local.Squid`))
  (`/Game/Squid/BP_Squid.Hide Ring` (`local.Squid`) false))

(fn `Damage Mermaid`
  ;[1 1 1] Check for Enough Live
  (if (== (`self.NbSquid`) 0)
    (`self.Set Current State` "NewEnumerator3")
    (else
      ;[1 1 1] Damage
      (`/Engine/EditorBlueprintResources/StandardMacros.DecrementInt` (`self.NbSquid`)
        (:`  `
          (`self.OnSquidPlaced`))))))

(fn `PlaceSquid`
  (params (Pedestal :type "/Game/Squid/BP_Pedestal Object Reference") (`Pedestal Occupied` :type Boolean))
  (bind _returnvalue (`self.GetTransform` (`local.Pedestal`)))
  (switch `/Game/Scripts/LevelState` (`self.CurrentState`)
    (:`NewEnumerator1`
      _)
    (:`NewEnumerator2`
      _))
  ;[1 1 1] Check Mode
  (switch `/Game/Scripts/ClickMode` (`self.CurrentMode`)
    (:`NewEnumerator0`
      ;[1 1 1] Check Placed
      (if (`local.Pedestal Occupied`)
        (`KismetSystemLibrary.PrintString` "Squid already placed")
        (else
          ;[1 1 1] Check NbSquid
          (if (<= (`self.NbSquid`) 0)
            (`KismetSystemLibrary.PrintString` "No more Squid")
            (else
              ;[1 1 1] Spawn Actor
              (`|SpawnActorFromClass` (`self.SquidPrefab`) (`KismetMathLibrary.MakeTransform` (`KismetMathLibrary.MakeVector` (.x (.location _returnvalue)) (.y (.location _returnvalue)) (+ (.z (.location _returnvalue)) (`/Game/Squid/BP_Pedestal.SquidOffset` (`local.Pedestal`)))) (.rotation _returnvalue) (.scale _returnvalue)) "Undefined" "OverrideRootScale" null null)
              (`/Engine/EditorBlueprintResources/StandardMacros.DecrementInt` (`self.NbSquid`)
                (:`  `
                  (`self.OnSquidPlaced`))))))))))

(fn `Set Camera`
  (params (Cam :type "Actor Object Reference"))
  (bind _output_get (set `self.Cam` Cam))
  (`PlayerController.SetViewTargetWithBlend` (`GameplayStatics.GetPlayerController` 0) _output_get 0.0 "VTBlend_Linear" 0.0 false))

(fn `Set Current State`
  (params (CurrentState :type "/Game/Scripts/LevelState Enum" :default "NewEnumerator0"))
  (set `self.PreviousState` (`self.CurrentState`))
  (set `self.CurrentState` CurrentState)
  (`self.OnLevelStateChanged`)
  (switch `/Game/Scripts/LevelState` (`self.CurrentState`)
    (:`NewEnumerator0`
      _)
    (:`NewEnumerator4`
      _)
    (:`NewEnumerator3`
      _))
  (`self.Change Mode` "NewEnumerator3"))

(fn `SetSquidColor`
  (params (Squid :type "/Game/Squid/BP_Squid Object Reference"))
  (bind _squid (`local.Squid`))
  (bind _selectedpearl_colorname (break `/Game/Scripts/ColorStruct` (`self.SelectedPearl`)))
  (bind _squidcolor_colorname (break `/Game/Scripts/ColorStruct` (`/Game/Squid/BP_Squid.SquidColor` _squid)))
  (switch `/Game/Scripts/LevelState` (`self.CurrentState`)
    (:`NewEnumerator1`
      _)
    (:`NewEnumerator2`
      _))
  (switch `/Game/Scripts/ClickMode` (`self.CurrentMode`)
    (:`NewEnumerator3`
      (`self.ControlSquid` Squid :!label _label))
    (:`NewEnumerator0`
      (goto _label))
    (:`NewEnumerator1`
      (if (not (== _selectedpearl_colorname _squidcolor_colorname))
        (`/Game/Squid/BP_Squid.Set Squid Color` _squid (`self.SelectedPearl`))
        (set `/Game/Squid/BP_Squid.Charge` 0.0 _squid)
        (`self.OnPearlSet`))
      (`self.ControlSquid` _squid))
    (:`NewEnumerator2`
      (goto _label))))

(fn `ShootShark`
  (params (ShootedShark :type "/Game/Shark/BP_Shark Object Reference") (DesireColor :type "/Game/Scripts/ColorStruct Structure"))
  (returns (ShootState :type "/Game/Scripts/Shootstate Enum"))
  (bind _selectedsquidcolor_colorname (break `/Game/Scripts/ColorStruct` (`self.SelectedSquidColor`)))
  (bind _squidcontrol (`self.SquidControl`))
  (bind _squidcontrol_2 (`self.SquidControl`))
  (bind _selectedsquidcolor_colorname_2 (break `/Game/Scripts/ColorStruct` (`self.SelectedSquidColor`)))
  (bind _squidcontrol_3 (`self.SquidControl`))
  (bind _squidcontrol_4 (`self.SquidControl`))
  (bind _desirecolor_colorname (break `/Game/Scripts/ColorStruct` (`local.DesireColor`)))
  (switch `/Game/Scripts/LevelState` (`self.CurrentState`)
    (:`NewEnumerator0`
      _)
    (:`NewEnumerator1`
      (switch `/Game/Scripts/ClickMode` (`self.CurrentMode`) :!label _label
        (:`NewEnumerator3`
          _)
        (:`NewEnumerator0`
          _)
        (:`NewEnumerator1`
          _)
        (:`NewEnumerator2`
          (if (== _selectedsquidcolor_colorname "None")
            (return "NewEnumerator3")
            (else
              ;[1 1 1] Check for Special Shoot
              (if (>= (`/Game/Squid/BP_Squid.Charge` _squidcontrol_4) (`/Game/Squid/BP_Squid.Max Charge` _squidcontrol_4))
                (set `/Game/Squid/BP_Squid.Charge` (- (`/Game/Squid/BP_Squid.Charge` _squidcontrol_3) (`/Game/Squid/BP_Squid.SpecialShootCost` _squidcontrol_3)) _squidcontrol_3)
                (else
                  ;[1 1 1] Check Range
                  (if (< (`KismetMathLibrary.Vector_Distance` (`self.K2_GetActorLocation` (`self.SquidControl`)) (`self.K2_GetActorLocation` (`local.ShootedShark`))) (`/Game/Squid/BP_Squid.Range` (`self.SquidControl`)))
                    ;[1 1 1] Check Charges
                    (if (> (`/Game/Squid/BP_Squid.Charge` _squidcontrol) (`/Game/Squid/BP_Squid.ShootCost` _squidcontrol))
                      (set `/Game/Squid/BP_Squid.Charge` (- (`/Game/Squid/BP_Squid.Charge` _squidcontrol_2) (`/Game/Squid/BP_Squid.ShootCost` _squidcontrol_2)) _squidcontrol_2)
                      (else
                        (return "NewEnumerator4")))
                    (else
                      (return "NewEnumerator1")))))
              ;[1 1 1] Check Color Match
              (if (== _desirecolor_colorname _selectedsquidcolor_colorname_2)
                (return "NewEnumerator0")
                (else
                  (return "NewEnumerator5")))))))
      (return "NewEnumerator2"))
    (:`NewEnumerator2`
      (goto _label))
    (:`NewEnumerator5`
      _)
    (:`NewEnumerator4`
      _)
    (:`NewEnumerator3`
      _))
  (return "NewEnumerator6"))

(fn `UserConstructionScript`)