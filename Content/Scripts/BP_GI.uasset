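; BP_GI, apparently the Game Instance, manages top-level UI switching, the level instance reference and quitting the game.
; SetUMG maps a game state (Main, Level, Game, Credit) to its HUD widget, adding a new one to the viewport and removing the previous CurrentUI.
; SetLevelInstance stores the passed level instance and calls OnLevelInstanceCreated to announce it.
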(fn `Quit`
  (`KismetSystemLibrary.QuitGame` null "Quit"))

(fn `Set Level Instance`
  (params (`Level Instance` :type "/Game/Scripts/BP_LI Object Reference"))
  (set `self.Level Instance` `Level Instance`)
  (`self.OnLevelInstanceCreated`))

(fn `SetUMG`
  (params (`New GameState` :type "/Game/HUD/UIEnum Enum" :default "NewEnumerator0"))
  (switch `/Game/HUD/UIEnum` `New GameState`
    (:`NewEnumerator0`
      (bind _returnvalue (`|CreateWidget` "/Game/HUD/UMG_MainMenu_HUD.UMG_MainMenu_HUD_C"))
      (`UserWidget.AddToViewport` _returnvalue 0)
      (if (`KismetSystemLibrary.IsValid` (`self.currentUI`))
        (`Widget.RemoveFromParent` (`self.currentUI`)))
      (set `self.currentUI` _returnvalue))
    (:`NewEnumerator1`
      (bind _returnvalue_2 (`|CreateWidget` "/Game/HUD/UMG_LevelSelect_HUD.UMG_LevelSelect_HUD_C"))
      (`UserWidget.AddToViewport` _returnvalue_2 0)
      (if (`KismetSystemLibrary.IsValid` (`self.currentUI`))
        (`Widget.RemoveFromParent` (`self.currentUI`)))
      (set `self.currentUI` _returnvalue_2))
    (:`NewEnumerator2`
      (bind _returnvalue_3 (`|CreateWidget` "/Game/HUD/UMG_Player_HUD.UMG_Player_HUD_C"))
      (`UserWidget.AddToViewport` _returnvalue_3 0)
      (if (`KismetSystemLibrary.IsValid` (`self.currentUI`))
        (`Widget.RemoveFromParent` (`self.currentUI`)))
      (set `self.currentUI` _returnvalue_3))
    (:`NewEnumerator3`
      (bind _returnvalue_4 (`|CreateWidget` "/Game/HUD/UMG_Credit_HUD.UMG_Credit_HUD_C"))
      (`UserWidget.AddToViewport` _returnvalue_4 0)
      (if (`KismetSystemLibrary.IsValid` (`self.currentUI`))
        (`Widget.RemoveFromParent` (`self.currentUI`)))
      (set `self.currentUI` _returnvalue_4))))