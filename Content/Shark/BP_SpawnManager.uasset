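; BP_SpawnManager spawns BP_Shark actors on a timed schedule and hands each to a path.
; BeginPlay insertion-sorts SpawnList by SpawnTime.
; Tick compares the current entry to time since creation, spawning at most one shark per frame, setting its color and adding it to the indexed entry in Paths.
; The manager destroys itself after spawning the last entry.
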(event `self.ReceiveBeginPlay`
  ;[1 1 1] Tri insertion, non optimisé
  (`self.Sort List`))

(event `self.ReceiveTick`
  (params (DeltaSeconds :type "Float (single-precision)"))
  (bind (_output_spawntime _output_path _output_sharktype _output_sharkcolor) (break `/Game/Scripts/SpawnStruct` (`self.Get Current`)))
  (bind _output_spawntime_2 (break `/Game/Scripts/SpawnStruct` (`self.Get Current`)))
  ;[1 1 1] Check Current SpawnTime
  (if (<= _output_spawntime_2 (`self.GetGameTimeSinceCreation`))
    ;[1 1 1] Spawn Shark
    (bind _returnvalue (`|SpawnActorFromClass` "/Game/Shark/BP_Shark.BP_Shark_C" (`self.OutRangeTransform`) "Undefined" "OverrideRootScale" null null))
    ;[1 1 1] Init Shark
    (set `/Game/Shark/BP_Shark.ColorName` _output_sharkcolor _returnvalue) ; Peut-être que Set une ColorStruct serait plus pertinant ?
    (`/Game/Shark/BP_Shark.Set Desired Color` _returnvalue)
    (`/Game/Shark/BP_Path.Add Shark` (`|GetArrayItem` (`self.Paths`) _output_path) _returnvalue)
    ;[1 1 1] Check for Next SharkToSpawn
    (if (< (`self.Current`) (- (`KismetArrayLibrary.Array_Length` (`self.SpawnList`)) 1))
      (`/Engine/EditorBlueprintResources/StandardMacros.IncrementInt` (`self.Current`))
      (else
        (`self.K2_DestroyActor`)))))

(fn `Sort List`
  (locals (j :type Integer))
  (bind _spawnlist (`self.SpawnList`))
  (bind _j (`local.j`))
  (bind _j_2 (`local.j`))
  (bind _output_spawntime (break `/Game/Scripts/SpawnStruct` (`|GetArrayItem` _spawnlist _j)))
  (bind _output_spawntime_2 (break `/Game/Scripts/SpawnStruct` (`|GetArrayItem` _spawnlist (- _j 1))))
  (for _index (range 1 (`KismetArrayLibrary.Array_Length` _spawnlist))
    (bind _output_get (set `local.j` _index))
    (while (and (> _output_get 0) (< _output_spawntime _output_spawntime_2))
      (`KismetArrayLibrary.Array_Swap` (`self.SpawnList`) _j_2 (- _j_2 1))
      (`/Engine/EditorBlueprintResources/StandardMacros.DecrementInt` (`local.j`)))))

(fn `UserConstructionScript`)