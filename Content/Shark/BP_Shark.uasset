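; Shark target that the player's squid fills by holding a click with a matching color, shown as kanji from a data table.
; Tick outlines it using range and screen-space cursor checks, then advances fill materials by shot type.
; A full shark leaves its path and is destroyed.
; Mismatched shots raise anger and speed, eventually triggering an angry dash flagged unkillable.
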(event `self.ReceiveBeginPlay`
  (`MeshComponent.SetScalarParameterValueOnMaterials` (`self.FillBar`) "Progression" 0.0)
  (`self.EnableInput` (`GameplayStatics.GetPlayerController` 0))
  ;[1 1 1] Set Level Instance
  (bind _asbp_gi (cast `/Game/Scripts/BP_GI` (`GameplayStatics.GetGameInstance`)))
  (`/Engine/EditorBlueprintResources/StandardMacros.IsValid` (`/Game/Scripts/BP_GI.Level Instance` _asbp_gi)
    (:`Is Valid`
      (`self.OnLICreated`))
    (:`Is Not Valid`
      (add `/Game/Scripts/BP_GI.OnLevelInstanceCreated` _asbp_gi (delegate `OnLICreated`)))))

(event `OnLICreated`
  ;[1 1 1] Set Level Instance
  (bind _asbp_gi (cast `/Game/Scripts/BP_GI` (`GameplayStatics.GetGameInstance`)))
  (set `self.Level Instance` (`/Game/Scripts/BP_GI.Level Instance` _asbp_gi)))

(event `self.ReceiveTick`
  (params (DeltaSeconds :type "Float (single-precision)"))
  (bind (_desire_color_colorname _desire_color_colorvector) (break `/Game/Scripts/ColorStruct` (`self.Desire color`)))
  (bind _fillbar (`self.FillBar`))
  (bind _returnvalue (`KismetMathLibrary.FClamp` (`self.Fillometer`)))
  (bind _controlledsquid (`/Game/Scripts/BP_LI.ControlledSquid` (`self.Level Instance`)))
  (bind _controlledsquid_2 (`/Game/Scripts/BP_LI.ControlledSquid` (`self.Level Instance`)))
  (bind _normal_shot_speed (`/Game/Squid/BP_Squid.Normal Shot Speed` _controlledsquid_2))
  (`|ExecutionSequence`
    (:`then_0`
      ;[1 1 1] Check Outline
      (`/Engine/EditorBlueprintResources/StandardMacros.IsValid` _controlledsquid
        (:`Is Valid`
          (bind _inrange (`self.CheckClickRange`))
          (if _inrange
            (if (< (`/Game/Squid/BP_Squid.Charge` _controlledsquid) 3.0)
              (if (< (`KismetMathLibrary.Vector_Distance` (`self.K2_GetActorLocation` _controlledsquid) (`self.K2_GetActorLocation`)) (`/Game/Squid/BP_Squid.Range` _controlledsquid))
                (`PrimitiveComponent.SetRenderCustomDepth` (`self.Shark`) true :!label _label)
                (`/Game/Scripts/BP_LI.ChangeCursorSize` (`self.Level Instance`) "Big")
                (else
                  (`PrimitiveComponent.SetRenderCustomDepth` (`self.Shark`) false :!label _label_2)
                  (`/Game/Scripts/BP_LI.ChangeCursorSize` (`self.Level Instance`) "Small")))
              (else
                (goto _label)))
            (else
              (goto _label_2))))))
    (:`then_1`
      (if (`self.Shooting`)
        (switch `/Game/Squid/SquidState` (`/Game/Squid/BP_Squid.CurrentState` _controlledsquid_2)
          (:`NewEnumerator2`
            ;[1 1 1] Normal Shot
            (set `self.Fillometer` (+ (`self.Fillometer`) (* (`self.Fill Speed Ratio`) _normal_shot_speed DeltaSeconds))))
          (:`NewEnumerator1`
            ;[1 1 1] Special Shot
            (set `self.Fillometer` (+ (`self.Fillometer`) (* (`self.Fill Speed Ratio`) _normal_shot_speed DeltaSeconds (`/Game/Squid/BP_Squid.Special Shot Ratio` _controlledsquid_2))))))
        (`|ExecutionSequence`
          (:`then_0`
            ;[1 1 1] Check if click still in range
            (bind _inrange_2 (`self.CheckClickRange`))
            (`PrimitiveComponent.SetRenderCustomDepth` (`self.Shark`) _inrange_2)
            (if _inrange_2
              (`/Game/Scripts/BP_LI.ChangeCursorSize` (`self.Level Instance`) "Big")
              (else
                (set `self.Shooting` false)
                (`/Game/Scripts/BP_LI.Stop Shooting` (`self.Level Instance`))
                (`/Game/Scripts/BP_LI.ChangeCursorSize` (`self.Level Instance`) "Small"))))
          (:`then_1`
            ;[1 1 1] Update Material
            (`MeshComponent.SetScalarParameterValueOnMaterials` _fillbar "Progression" _returnvalue)
            (`MeshComponent.SetVectorParameterValueOnMaterials` _fillbar "Color" _desire_color_colorvector)
            (`MeshComponent.SetVectorParameterValueOnMaterials` (`self.Shark`) "Color" (- (+ _desire_color_colorvector (1.0 1.0 1.0)) (`KismetMathLibrary.MakeVector` _returnvalue _returnvalue _returnvalue)))
            ;[1 1 1] Check if color is filled
            (if (>= (`self.Fillometer`) 1.0)
              (`/Game/Scripts/BP_LI.Stop Shooting` (`self.Level Instance`))
              (`/Game/Shark/BP_Path.Remove Shark` (`self.Path`) self)
              (`KismetSystemLibrary.Delay` 1.0)
              (`self.K2_DestroyActor`))))))))

(event `self.Shark.OnClicked`
  (params (TouchedComponent :type "PrimitiveComponent Object Reference") (ButtonPressed :type "Key Structure"))
  ;[1 1 1 0.5 78] Handle Click
  (bind _shootstate (`/Game/Scripts/BP_LI.Shoot Shark` (`self.Level Instance`) self (`self.Desire color`)))
  (switch `/Game/Scripts/Shootstate` _shootstate
    (:`NewEnumerator0`
      (set `self.Shooting` true))
    (:`NewEnumerator5`
      ;;[1 1 1] Handle Angriness
      (bind _result (`/Engine/EditorBlueprintResources/StandardMacros.IncrementInt` (`self.Angriness`))
        (:`  `
          (if (> _result (`self.Max angriness`))
            (if (not (`self.Unkillable`))
              ;;[1 1 1] Dash
              (set `self.Unkillable` true)
              (set `self.Speed` 100.0)
              (bind _asab_shark (cast `/Game/Shark/AB_Shark` (`SkeletalMeshComponent.GetAnimInstance` (`self.Shark`))))
              (set `/Game/Shark/AB_Shark.IsMovingAngry` true _asab_shark))
            (else
              ;;[1 1 1] Boost Speed
              (set `self.Speed` (+ (`self.Speed`) (`self.BoostSpeed`))))))))))

(event `Key|LeftMouseButton`
  (params (Key :type "Key Structure"))
  ;[1 1 1 0.5 78] Handle Click
  (:`Released`
    (set `self.Shooting` false :!label _label_3)
    (`/Game/Scripts/BP_LI.Stop Shooting` (`self.Level Instance`))))

(event `self.Shark.OnReleased`
  (params (TouchedComponent :type "PrimitiveComponent Object Reference") (ButtonReleased :type "Key Structure"))
  ;[1 1 1 0.5 78] Handle Click
  (goto _label_3))

(fn `Set Desired Color`
  (params (RowName :type Name))
  (bind (_desire_color_colorname _desire_color_colorvector _desire_color_kanji) (break `/Game/Scripts/ColorStruct` (`self.Desire color`)))
  ;[1 1 1] Set Desired Color
  (bind _returnvalue (`|GetDataTableRow` (`self.Data`) RowName)
    (:`then`
      (set `self.Desire color` _returnvalue)
      ;[1 1 1] Display Kanji
      (bind _returnvalue_2 (`DecalComponent.CreateDynamicMaterialInstance` (`self.KanjiLeft`)))
      (`MaterialInstanceDynamic.SetTextureParameterValue` _returnvalue_2 "Kanji" _desire_color_kanji)
      (bind _returnvalue_3 (`DecalComponent.CreateDynamicMaterialInstance` (`self.KanjiRight`)))
      (`MaterialInstanceDynamic.SetTextureParameterValue` _returnvalue_3 "Kanji" _desire_color_kanji))
    (:`RowNotFound`
      (`KismetSystemLibrary.PrintString` "Row Not Found" true true (struct :`G` 0.66 :`B` 1.0 :`A` 1.0) 0.0))))

(fn `UserConstructionScript`)