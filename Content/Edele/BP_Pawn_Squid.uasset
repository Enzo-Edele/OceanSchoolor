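; BP_Pawn_Squid is a clickable squid pawn that can be recolored or taken control of through the game instance.
; On BeginPlay it sets the player's view to its camera and enables mouse clicks.
; Tick builds a reload Charge up to about three seconds, printing it as it rises.
; Clicking its Cube asks BP_GI to set its color; failing that, BP_GI gives control and switches to shot mode with SquidColor.
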(event `self.ReceiveBeginPlay`
  (bind _returnvalue (`GameplayStatics.GetPlayerController` 0))
  (`PlayerController.SetViewTargetWithBlend` (`GameplayStatics.GetPlayerController` 0) (`self.Camera`) 0.0 "VTBlend_Linear" 0.0 false)
  (set `PlayerController.bEnableClickEvents` true _returnvalue)
  (set `PlayerController.bShowMouseCursor` true _returnvalue))

(event `self.ReceiveTick`
  (params (DeltaSeconds :type "Float (single-precision)"))
  (if (< (`self.Charge`) 3.0)
    (bind _output_get (set `self.Charge` (+ (`self.Charge`) DeltaSeconds)))
    (`KismetSystemLibrary.PrintString` (`KismetStringLibrary.Conv_DoubleToString` _output_get) true true (struct :`G` 0.66 :`B` 1.0 :`A` 1.0) 0.0)))

(event `self.Cube.OnClicked`
  (params (TouchedComponent :type "PrimitiveComponent Object Reference") (ButtonPressed :type "Key Structure"))
  (`KismetSystemLibrary.PrintString` "Click squid")
  (bind _asbp_gi (cast `/Game/Edele/BP_GI` (`GameplayStatics.GetGameInstance`)))
  (bind _changed (`/Game/Edele/BP_GI.SetSquidColor` _asbp_gi self))
  (if _changed
    (`KismetSystemLibrary.PrintString` "Change Color")
    (else
      (`/Game/Edele/BP_GI.ControlSquid` _asbp_gi self)
      (`/Game/Edele/BP_GI.ChangeMode` _asbp_gi false false true (`self.SquidColor`))
      (`KismetSystemLibrary.PrintString` "Change Control"))))

(fn `UserConstructionScript`)