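; BP_GI, by its name a game instance, holds the squid, pearl and shot mode flags for a game with squids, pearls and sharks.
; ChangeMode sets all three flags at once.
; SetSquidColor applies a pearl color to a BP_Pawn_Squid only while pearl mode is on.
; PlaceSquid, ControlSquid and ShotShark are empty stubs.
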(fn `ChangeMode`
  (params (SquidMode :type Boolean) (PearlMode :type Boolean) (ShotMode :type Boolean))
  (set `self.SquidMode` SquidMode)
  (set `self.PearlMode` PearlMode)
  (set `self.ShotMode` ShotMode))

(fn `ControlSquid`
  (params (Squid :type "Actor Object Reference")))

(fn `PlaceSquid`)

(fn `SetSquidColor`
  (params (PearlColor :type "Color Structure") (Squid :type "Actor Object Reference"))
  (returns (Changed :type Boolean))
  (if (`self.PearlMode`)
    (bind _asbp_pawn_squid (cast `/Game/Edele/BP_Pawn_Squid` (`local.Squid`)))
    (set `/Game/Edele/BP_Pawn_Squid.SquidColor` PearlColor _asbp_pawn_squid)
    (return (`self.PearlMode`))))

(fn `ShotShark`)