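; Mermaid actor that offers red, green and blue pearls to click, passing the chosen color's data-table row to the level instance through a mode change.
; It registers with the level instance once created and feeds the squid count to a Niagara system whenever a squid is placed.
; When a pearl is set during WaveIncoming, that color's timeline, rate-scaled to the cooldown, animates its dynamic material and blocks clicks until finished.
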(event `self.ReceiveBeginPlay`
  (bind _asbp_gi (cast `/Game/Scripts/BP_GI` (`GameplayStatics.GetGameInstance`)))
  (`/Engine/EditorBlueprintResources/StandardMacros.IsValid` (`/Game/Scripts/BP_GI.Level Instance` _asbp_gi)
    (:`Is Valid`
      (`self.OnLICreated`))
    (:`Is Not Valid`
      (add `/Game/Scripts/BP_GI.OnLevelInstanceCreated` _asbp_gi (delegate `OnLICreated`)))))

(event `OnLICreated`
  (bind _asbp_gi (cast `/Game/Scripts/BP_GI` (`GameplayStatics.GetGameInstance`)))
  (bind _output_get (set `self.Level Instance` (`/Game/Scripts/BP_GI.Level Instance` _asbp_gi)))
  (set `/Game/Scripts/BP_LI.Mermaid` self _output_get)
  (add `/Game/Scripts/BP_LI.OnSquidPlaced` (`self.Level Instance`) (delegate `Update Niagara`))
  (add `/Game/Scripts/BP_LI.OnPearlSet` (`self.Level Instance`) (delegate `OnPearlSet`))
  (`self.Update Niagara`)
  (`self.Create Pearl Dynamic Mats`))

(event `Update Niagara`
  (bind _ns_squid (`self.NS_Squid`))
  ;[1 1 1] Update VFX
  (`NiagaraComponent.SetVariableInt` _ns_squid "NbSquid" (`/Game/Scripts/BP_LI.NbSquid` (`self.Level Instance`)))
  (`NiagaraComponent.ReinitializeSystem` _ns_squid))

(event `OnPearlSet`
  (bind _level_instance (`self.Level Instance`))
  (bind _selectedpearl_colorname (break `/Game/Scripts/ColorStruct` (`/Game/Scripts/BP_LI.SelectedPearl` _level_instance)))
  (bind _colorcooldown (`/Game/Scripts/BP_LI.ColorCoolDown` (`self.Level Instance`)))
  ;[1 1 1] On Pearl Set
  (if (`KismetStringLibrary.EqualEqual_StrStr` "WaveIncoming" (`|GetEnumeratorNameAsString` (`/Game/Scripts/BP_LI.CurrentState` _level_instance)))
    (switch `name` _selectedpearl_colorname
      (:`Red`
        (`KismetArrayLibrary.Array_Set` (`self.PearlCD`) 0 true)
        (`TimelineComponent.SetPlayRate` (`self.Progression R`) (/ 1.0 _colorcooldown))
        (bind (_direction _progression) (`Timeline|Progression R` :!via `PlayFromStart`)
          (:`Update`
            (`MaterialInstanceDynamic.SetScalarParameterValue` (`|GetArrayItem` (`self.M_Pearl`)) "Progression" _progression))
          (:`Finished`
            (`KismetArrayLibrary.Array_Set` (`self.PearlCD`)))))
      (:`Green`
        (`KismetArrayLibrary.Array_Set` (`self.PearlCD`) 1 true)
        (`TimelineComponent.SetPlayRate` (`self.Progression G`) (/ 1.0 _colorcooldown))
        (bind (_direction_2 _progression_2) (`Timeline|Progression G` :!via `PlayFromStart`)
          (:`Update`
            (`MaterialInstanceDynamic.SetScalarParameterValue` (`|GetArrayItem` (`self.M_Pearl`) 1) "Progression" _progression_2))
          (:`Finished`
            (`KismetArrayLibrary.Array_Set` (`self.PearlCD`) 1))))
      (:`Blue`
        (`KismetArrayLibrary.Array_Set` (`self.PearlCD`) 2 true)
        (`TimelineComponent.SetPlayRate` (`self.Progression B`) (/ 1.0 _colorcooldown))
        (bind (_direction_3 _progression_3) (`Timeline|Progression B` :!via `PlayFromStart`)
          (:`Update`
            (`MaterialInstanceDynamic.SetScalarParameterValue` (`|GetArrayItem` (`self.M_Pearl`) 2) "Progression" _progression_3))
          (:`Finished`
            (`KismetArrayLibrary.Array_Set` (`self.PearlCD`) 2)))))))

(event `self.RedBox.OnClicked`
  (params (TouchedComponent :type "PrimitiveComponent Object Reference") (ButtonPressed :type "Key Structure"))
  (if (not (`|GetArrayItem` (`self.PearlCD`)))
    (bind _returnvalue (`|GetDataTableRow` (`self.Data`) "Red")
      (:`then`
        (`self.Set Pearl` _returnvalue)))))

(event `self.GreenBox.OnClicked`
  (params (TouchedComponent :type "PrimitiveComponent Object Reference") (ButtonPressed :type "Key Structure"))
  (if (not (`|GetArrayItem` (`self.PearlCD`) 1))
    (bind _returnvalue (`|GetDataTableRow` (`self.Data`) "Green")
      (:`then`
        (`self.Set Pearl` _returnvalue)))))

(event `self.BlueBox.OnClicked`
  (params (TouchedComponent :type "PrimitiveComponent Object Reference") (ButtonPressed :type "Key Structure"))
  (if (not (`|GetArrayItem` (`self.PearlCD`) 2))
    (bind _returnvalue (`|GetDataTableRow` (`self.Data`) "Blue")
      (:`then`
        (`self.Set Pearl` _returnvalue)))))

(fn `Create Pearl Dynamic Mats`
  (bind _redpearl (`self.RedPearl`))
  (bind _greenpearl (`self.GreenPearl`))
  (bind _bluepearl (`self.BluePearl`))
  (`|ExecutionSequence`
    (:`then_0`
      (bind _returnvalue (`PrimitiveComponent.CreateDynamicMaterialInstance` _redpearl 0 null (`KismetStringLibrary.Conv_StringToName` (`KismetSystemLibrary.GetObjectName` _redpearl))))
      (`KismetArrayLibrary.Array_Add` (`self.M_Pearl`) _returnvalue))
    (:`then_1`
      (bind _returnvalue_2 (`PrimitiveComponent.CreateDynamicMaterialInstance` _greenpearl 0 null (`KismetStringLibrary.Conv_StringToName` (`KismetSystemLibrary.GetObjectName` _greenpearl))))
      (`KismetArrayLibrary.Array_Add` (`self.M_Pearl`) _returnvalue_2))
    (:`then_2`
      (bind _returnvalue_3 (`PrimitiveComponent.CreateDynamicMaterialInstance` _bluepearl 0 null (`KismetStringLibrary.Conv_StringToName` (`KismetSystemLibrary.GetObjectName` _bluepearl))))
      (`KismetArrayLibrary.Array_Add` (`self.M_Pearl`) _returnvalue_3))))

(fn `Set Pearl`
  (params (Color :type "/Game/Scripts/ColorStruct Structure"))
  (`/Game/Scripts/BP_LI.Change Mode` (`self.Level Instance`) "NewEnumerator1" Color))

(fn `UserConstructionScript`)